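; Base enemy actor that follows a spline path, takes damage and awards gold when killed, as in a tower defense game.
; Each tick it advances a distance along PathSpline by MoveSpeed and matches the spline's location and rotation, stopping at the end.
; ApplyDamage lowers health set from MaxHealth at BeginPlay.
; At zero, Die adds EnemyGold to the GameState, updates the HUD and destroys the actor.
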(event Custom|ApplyDamage
  (params (DamageAmount :type Float%20%28double-precision%29))
  (bind _output_get (Variables|Default|SetCurrentHealth (- (stale _output_get) DamageAmount)))
  (if (<= _output_get 0.0)
    (CallFunction|Die)))

(event Custom|Die
  (Utilities|FlowControl|Sequence
    (:then_0
      (bind _asbp_my_hud (Utilities|Casting|CastToBP_MyHud (HUD|GetHUD (Game|GetPlayerController 0)))))
    (:then_1
      (bind _asbp_game_state (Utilities|Casting|CastToBP_GameState (Game|GetGameState))
        (:then
          (bind _output_get (Variables|/Game/Actors/BP_GameState.BP_GameState_C|SetGoldCount _asbp_game_state (+ (Variables|/Game/Actors/BP_GameState.BP_GameState_C|GetGoldCount _asbp_game_state) (Variables|Default|GetEnemyGold))))
          (Default|SetGold _asbp_my_hud _output_get))
        (:CastFailed
          (Development|PrintString "failed"))))
    (:then_2
      (Actor|DestroyActor)
      (Development|PrintString "dead"))))

(event EventBeginPlay
  (Variables|Default|SetCurrentHealth (Variables|Default|GetMaxHealth)))

(event EventTick
  (params (DeltaSeconds :type Float%20%28single-precision%29))
  (bind _pathspline (Variables|Components|GetPathSpline))
  (if (Utilities|IsValid (Variables|Components|GetPathSpline))
    (bind _output_get (Variables|Default|SetDistance (+ (Variables|Default|GetDistance) (* (Utilities|Time|GetWorldDeltaSeconds) (Variables|Default|GetMoveSpeed)))))
    (if (not (>= _output_get (Spline|GetSplineLength _pathspline)))
      (Transformation|SetActorLocationAndRotation (Spline|GetLocationatDistanceAlongSpline _pathspline (Variables|Default|GetDistance) "World") (Spline|GetRotationatDistanceAlongSpline _pathspline (Variables|Default|GetDistance) "World")))))

(fn ConstructionScript)