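; BP_EnemyParent is an enemy base actor that follows a spline path and awards gold on death.
; BeginPlay scales health by the GameState's wave difficulty; damage reaching zero health triggers Die, which destroys it and updates GameState and HUD gold.
; Tick advances distance along PathSpline using a speed multiplier set by ApplySlow.
; The slow expiry check is inverted, resetting speed while SlowEndTime is still in the future.
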(event Custom|ApplyDamage
  (params (DamageAmount :type Float%20%28double-precision%29))
  (bind _output_get (Variables|Default|SetCurrentHealth (- (stale _output_get) DamageAmount)))
  (if (<= _output_get 0.0)
    (CallFunction|Die)))

(event Custom|Die
  (Utilities|FlowControl|Sequence
    (:then_0
      (Actor|DestroyActor)
      (Development|PrintString "dead"))
    (:then_1
      (bind _asbp_my_hud (Utilities|Casting|CastToBP_MyHud (HUD|GetHUD (Game|GetPlayerController 0))))
      (bind _output_get (Variables|Default|SetAs%20BP%20My%20Hud _asbp_my_hud)))
    (:then_2
      (bind _asbp_game_state (Utilities|Casting|CastToBP_GameState (Game|GetGameState)))
      (bind _output_get_2 (Variables|/Game/Actors/UI_Assets/BP_GameState.BP_GameState_C|SetGoldCount _asbp_game_state (+ (Variables|/Game/Actors/UI_Assets/BP_GameState.BP_GameState_C|GetGoldCount _asbp_game_state) (Variables|Default|GetGoldCount))))
      (Default|SetGold _output_get _output_get_2))))

(event EventBeginPlay
  (bind _asbp_game_state (Utilities|Casting|CastToBP_GameState (Game|GetGameState)))
  (Variables|Default|SetCurrentHealth (* (Variables|/Game/Actors/UI_Assets/BP_GameState.BP_GameState_C|GetWaveDifficulty _asbp_game_state) (Variables|Default|GetBaseHealth))))

(event Collision|EventActorBeginOverlap
  (params (OtherActor :type Actor%20Object%20Reference)))

(event EventTick
  (params (DeltaSeconds :type Float%20%28single-precision%29))
  (bind _pathspline (Variables|Components|GetPathSpline))
  (if (Utilities|IsValid (Variables|Components|GetPathSpline))
    (if (and (< (Variables|Default|GetSpeedMultiplier) 1.0) (> (Variables|Default|GetSlowEndTime) (Utilities|Time|GetGameTimeinSeconds)))
      (Variables|Default|SetSpeedMultiplier 1.0))
    (bind _output_get (Variables|Default|SetDistance (+ (Variables|Default|GetDistance) (* (Utilities|Time|GetWorldDeltaSeconds) (* (Variables|Default|GetMoveSpeed) (Variables|Default|GetSpeedMultiplier))))))
    (if (not (>= _output_get (Spline|GetSplineLength _pathspline)))
      (Transformation|SetActorLocationAndRotation (Spline|GetLocationatDistanceAlongSpline _pathspline (Variables|Default|GetDistance) "World") (Spline|GetRotationatDistanceAlongSpline _pathspline (Variables|Default|GetDistance) "World")))))

(fn ConstructionScript)

(fn ApplySlow
  (params (SlowMultiplier :type Float%20%28double-precision%29) (Duration :type Float%20%28double-precision%29))
  (Variables|Default|SetSpeedMultiplier SlowMultiplier)
  (Variables|Default|SetSlowEndTime (+ (Utilities|Time|GetGameTimeinSeconds) Duration)))