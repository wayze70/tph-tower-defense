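; Enemy spawner actor that releases a wave of enemies at its own transform and assigns each a path spline.
; StartWave resets the count and starts a looping timer that calls SpawnOne at a set interval.
; SpawnOne maps the next entry in the selected wave to a fast, basic, big or boss class.
; The timer is never cleared here, and the difficulty input is unused.
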(event Custom|SpawnOne
  (if (< (Variables|Default|GetSpawnedCount) (Utilities|Array|Length (Variables|/Game/Actors/waves/Wave1.Wave1_C|GetWave (Utilities|Array|Get(acopy) (Variables|Default|GetWaves) (stale Custom|StartWave WaveNum)))))
    (switch int (Utilities|Array|Get(acopy) (Variables|/Game/Actors/waves/Wave1.Wave1_C|GetWave (Utilities|Array|Get(acopy) (Variables|Default|GetWaves) (stale Custom|StartWave WaveNum))) (Variables|Default|GetSpawnedCount))
      (:0
        (Variables|Default|SetEnemyClass (Variables|Default|GetEnemyFast)))
      (:1
        (Variables|Default|SetEnemyClass (Variables|Default|GetEnemyBasic)))
      (:2
        (Variables|Default|SetEnemyClass (Variables|Default|GetEnemyBig)))
      (:3
        (Variables|Default|SetEnemyClass (Variables|Default|GetEnemyBoss))))
    (bind _returnvalue (Game|SpawnActorfromClass (Variables|Default|GetEnemyClass) (Math|Transform|MakeTransform (Transformation|GetActorLocation) (Transformation|GetActorRotation)) "Undefined" "MultiplyWithRoot" 0 0))
    (Development|PrintString (Utilities|GetDisplayName _returnvalue))
    (Variables|/Game/Actors/BP_EnemyParent.BP_EnemyParent_C|SetPathSpline _returnvalue (Variables|/Game/Actors/BP_Path.BP_Path_C|GetPathSpline (Variables|Default|GetPathSpline)))
    (Variables|Default|SetSpawnedCount (+ (Variables|Default|GetSpawnedCount) 1))))

(event Custom|StartWave
  (params (WaveNum :type Integer) (WafeDifficulty :type Float%20%28double-precision%29))
  (Variables|Default|SetSpawnedCount 0)
  (Development|PrintString (Utilities|GetDisplayName (Utilities|Array|Get(acopy) (Variables|Default|GetWaves) WaveNum)))
  (bind _returnvalue (Utilities|Time|SetTimerbyFunctionName 0 "SpawnOne" (Variables|Default|GetSpawnInterval) true))
  (Variables|Default|SetSpawnTimerHandle _returnvalue))

(event EventBeginPlay)

(event Collision|EventActorBeginOverlap
  (params (OtherActor :type Actor%20Object%20Reference)))

(event EventTick
  (params (DeltaSeconds :type Float%20%28single-precision%29)))

(fn ConstructionScript)