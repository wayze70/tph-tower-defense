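; BP_MainBase is the player's base (tower) that loses health when enemies overlap it.
; BeginPlay caches the HUD, game state and player controller.
; On overlap with a BP_EnemyParent, it subtracts that enemy's TowerDamage from the game state's TowerHealth, updates the HUD and destroys the enemy.
; At zero health or below, it calls XPressed on the player controller; debug prints report collisions and remaining health.
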(event EventBeginPlay
  (Utilities|FlowControl|Sequence
    (:then_0
      (bind _asbp_my_hud (Utilities|Casting|CastToBP_MyHud (HUD|GetHUD (Game|GetPlayerController 0))))
      (Variables|Default|SetAs%20BP%20My%20Hud _asbp_my_hud))
    (:then_1
      (bind _asbp_game_state (Utilities|Casting|CastToBP_GameState (Game|GetGameState))))
    (:then_2
      (bind _asbp_third_person_player_controller (Utilities|Casting|CastToBP_ThirdPersonPlayerController (Game|GetPlayerController 0))))))

(event Collision|EventActorBeginOverlap
  (params (OtherActor :type Actor%20Object%20Reference))
  (Development|PrintString "colided")
  (bind _asbp_enemy_parent (Utilities|Casting|CastToBP_EnemyParent OtherActor))
  (bind _output_get (Variables|Default|SetAs%20BP%20Enemy%20Base _asbp_enemy_parent))
  (bind _output_get_2 (Variables|/Game/Actors/BP_GameState.BP_GameState_C|SetTowerHealth (stale EventBeginPlay _asbp_game_state) (- (Variables|/Game/Actors/BP_GameState.BP_GameState_C|GetTowerHealth (stale EventBeginPlay _asbp_game_state)) (Variables|/Game/Actors/BP_EnemyParent.BP_EnemyParent_C|GetTowerDamage _output_get))))
  (if (> _output_get_2 0)
    (Development|PrintString (Utilities|String|ToString(Integer) _output_get_2))
    (else
      (Default|XPressed (stale EventBeginPlay _asbp_third_person_player_controller))))
  (Default|SetTowerHealth (Variables|Default|GetAs%20BP%20My%20Hud) _output_get_2)
  (Actor|DestroyActor _output_get))

(event EventTick
  (params (DeltaSeconds :type Float%20%28single-precision%29)))

(fn ConstructionScript)