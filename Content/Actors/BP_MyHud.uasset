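; BP_MyHud is the game's UI manager, owning the gold counter, tower health display and main menu widgets.
; On BeginPlay it creates all three widgets and adds gold and tower health to the viewport, leaving the menu hidden.
; SetGold and SetTowerHealth forward values to their widgets, while ShowHideMainMenu toggles the menu by adding or removing it from the viewport.
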(event Custom|SetGold
  (params (Gold :type Integer))
  (Default|ChangeGold (Variables|Default|GetGoldCountGUI) Gold))

(event Custom|ShowHideMainMenu
  (bind _mainmenu (Variables|Default|GetMainMenu))
  (if (Widget|IsVisible (Variables|Default|GetMainMenu))
    (Widget|RemovefromParent _mainmenu)
    (else
      (UserInterface|Viewport|AddtoViewport _mainmenu 0))))

(event Custom|SetTowerHealth
  (params (TowerHealth :type Integer))
  (Default|ChangeTowerHealth (Variables|Default|GetTowerHealthGUI) TowerHealth))

(event EventBeginPlay
  (Utilities|FlowControl|Sequence
    (:then_0
      (bind _returnvalue (UserInterface|CreateWidget "/Game/Actors/WBP_Gold.WBP_Gold_C"))
      (bind _output_get (Variables|Default|SetGoldCountGUI _returnvalue))
      (UserInterface|Viewport|AddtoViewport _output_get 0))
    (:then_1
      (bind _returnvalue_2 (UserInterface|CreateWidget "/Game/Actors/WBP_MainMenu.WBP_MainMenu_C"))
      (Variables|Default|SetMainMenu _returnvalue_2))
    (:then_2
      (bind _returnvalue_3 (UserInterface|CreateWidget "/Game/Actors/WBP_TowerHealth.WBP_TowerHealth_C"))
      (bind _output_get_2 (Variables|Default|SetTowerHealthGUI _returnvalue_3))
      (UserInterface|Viewport|AddtoViewport _output_get_2 0))))

(event Collision|EventActorBeginOverlap
  (params (OtherActor :type Actor%20Object%20Reference)))

(event EventTick
  (params (DeltaSeconds :type Float%20%28single-precision%29)))

(fn ConstructionScript)