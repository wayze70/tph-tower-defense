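; BP_Projectile is a projectile actor that flies toward an assigned Target and damages enemies.
; On BeginPlay it aims its ProjectileMovement velocity once at the Target's current location, scaled by Speed, or destroys itself if the Target is invalid.
; When its collision sphere overlaps any BP_EnemyParent, not only the Target, it applies Damage to that enemy and destroys itself.
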(event OnComponentBeginOverlap(CollisionSphere)
  (params (OverlappedComponent :type Primitive%20Component%20Object%20Reference) (OtherActor :type Actor%20Object%20Reference) (OtherComp :type Primitive%20Component%20Object%20Reference) (OtherBodyIndex :type Integer) (bFromSweep :type Boolean) (SweepResult :type Hit%20Result%20Structure%20%28by%20ref%29))
  (bind _asbp_enemy_parent (Utilities|Casting|CastToBP_EnemyParent OtherActor))
  (Default|ApplyDamage _asbp_enemy_parent (Variables|Default|GetDamage))
  (Actor|DestroyActor))

(event EventBeginPlay
  (if (Utilities|IsValid (Variables|Default|GetTarget))
    (Variables|/Script/Engine.MovementComponent|SetVelocity (Variables|Default|GetProjectileMovement) (* (Math|Vector|Normalize (- (Transformation|GetActorLocation (Variables|Default|GetTarget)) (Transformation|GetActorLocation))) (Variables|Default|GetSpeed)))
    (else
      (Actor|DestroyActor))))

(event Collision|EventActorBeginOverlap
  (params (OtherActor :type Actor%20Object%20Reference)))

(event EventTick
  (params (DeltaSeconds :type Float%20%28single-precision%29)))

(fn ConstructionScript)