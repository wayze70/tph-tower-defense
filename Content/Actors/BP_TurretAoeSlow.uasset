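; BP_TurretAoeSlow is a turret that slows all enemies within its range.
; RangeSphere overlap events add and remove BP_EnemyParent actors in EnemiesInRange, without duplicates.
; A looping timer started on BeginPlay calls AoeSlow every TickInterval, applying a timed slow to each tracked enemy.
; The same pass removes invalid entries from the array while iterating over it.
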(event OnComponentBeginOverlap(RangeSphere)
  (params (OverlappedComponent :type Primitive%20Component%20Object%20Reference) (OtherActor :type Actor%20Object%20Reference) (OtherComp :type Primitive%20Component%20Object%20Reference) (OtherBodyIndex :type Integer) (bFromSweep :type Boolean) (SweepResult :type Hit%20Result%20Structure%20%28by%20ref%29))
  (bind _asbp_enemy_parent (Utilities|Casting|CastToBP_EnemyParent OtherActor))
  (Utilities|Array|AddUnique (Variables|Default|GetEnemiesInRange) _asbp_enemy_parent))

(event OnComponentEndOverlap(RangeSphere)
  (params (OverlappedComponent :type Primitive%20Component%20Object%20Reference) (OtherActor :type Actor%20Object%20Reference) (OtherComp :type Primitive%20Component%20Object%20Reference) (OtherBodyIndex :type Integer))
  (bind _asbp_enemy_parent (Utilities|Casting|CastToBP_EnemyParent OtherActor))
  (Utilities|Array|RemoveItem (Variables|Default|GetEnemiesInRange) _asbp_enemy_parent))

(event Custom|AoeSlow
  (bind _enemiesinrange (Variables|Default|GetEnemiesInRange))
  (for _array_element _enemiesinrange
    (if (Utilities|IsValid _array_element)
      (Default|ApplySlow _array_element (Variables|Default|GetSlowMultiplier) (Variables|Default|GetSlowDuration))
      (else
        (Utilities|Array|RemoveItem _enemiesinrange _array_element)))))

(event EventBeginPlay
  (Utilities|Time|SetTimerbyFunctionName 0 "AoeSlow" (Variables|Default|GetTickInterval) true))

(event Collision|EventActorBeginOverlap
  (params (OtherActor :type Actor%20Object%20Reference)))

(event EventTick
  (params (DeltaSeconds :type Float%20%28single-precision%29)))

(fn ConstructionScript
  (|CallParentFunction))