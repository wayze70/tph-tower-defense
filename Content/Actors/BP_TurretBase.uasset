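; Base turret actor that automatically attacks BP_EnemyBase actors within its range sphere.
; Sphere overlap events add and remove enemies from an EnemiesInRange list.
; A looping timer started on BeginPlay calls Fire every FireRate, which targets the first listed enemy, snaps the whole actor to face it and applies Damage directly, with no projectile.
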(event OnComponentBeginOverlap(RangeSphere)
  (params (OverlappedComponent :type Primitive%20Component%20Object%20Reference) (OtherActor :type Actor%20Object%20Reference) (OtherComp :type Primitive%20Component%20Object%20Reference) (OtherBodyIndex :type Integer) (bFromSweep :type Boolean) (SweepResult :type Hit%20Result%20Structure%20%28by%20ref%29))
  (bind _asbp_enemy_base (Utilities|Casting|CastToBP_EnemyBase OtherActor))
  (Utilities|Array|Add (Variables|Default|GetEnemiesInRange) _asbp_enemy_base))

(event OnComponentEndOverlap(RangeSphere)
  (params (OverlappedComponent :type Primitive%20Component%20Object%20Reference) (OtherActor :type Actor%20Object%20Reference) (OtherComp :type Primitive%20Component%20Object%20Reference) (OtherBodyIndex :type Integer))
  (bind _asbp_enemy_base (Utilities|Casting|CastToBP_EnemyBase OtherActor))
  (Utilities|Array|RemoveItem (Variables|Default|GetEnemiesInRange) _asbp_enemy_base))

(event Custom|Fire
  (bind _enemiesinrange (Variables|Default|GetEnemiesInRange))
  (if (> (Utilities|Array|Length (Variables|Default|GetEnemiesInRange)) 0)
    (bind _output_get (Variables|Default|SetCurrentTarget (Utilities|Array|Get(acopy) _enemiesinrange)))
    (if (Utilities|IsValid _output_get)
      (if (Utilities|Array|ContainsItem _enemiesinrange _output_get)
        (bind _asbp_enemy_base (Utilities|Casting|CastToBP_EnemyBase _output_get))
        (Transformation|SetActorRotation (Math|Rotator|FindLookatRotation (Transformation|GetActorLocation) (Transformation|GetActorLocation _asbp_enemy_base)))
        (Default|ApplyDamage _asbp_enemy_base (Variables|Default|GetDamage))))))

(event EventBeginPlay
  (Utilities|Time|SetTimerbyFunctionName 0 "Fire" (Variables|Default|GetFireRate) true))

(event Collision|EventActorBeginOverlap
  (params (OtherActor :type Actor%20Object%20Reference)))

(fn ConstructionScript)