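; BP_TurretSingle is a turret actor that automatically shoots one enemy at a time within its range.
; RangeSphere overlaps add and remove BP_EnemyParent actors in an EnemiesInRange list.
; A looping timer set on BeginPlay calls Fire every FireRate, snapping the whole actor to face the first listed enemy.
; It then spawns a BP_Projectile slightly above itself, passing Damage and that enemy as its target.
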(event OnComponentBeginOverlap(RangeSphere)
  (params (OverlappedComponent :type Primitive%20Component%20Object%20Reference) (OtherActor :type Actor%20Object%20Reference) (OtherComp :type Primitive%20Component%20Object%20Reference) (OtherBodyIndex :type Integer) (bFromSweep :type Boolean) (SweepResult :type Hit%20Result%20Structure%20%28by%20ref%29))
  (bind _asbp_enemy_parent (Utilities|Casting|CastToBP_EnemyParent OtherActor))
  (Utilities|Array|Add (Variables|Default|GetEnemiesInRange) _asbp_enemy_parent))

(event OnComponentEndOverlap(RangeSphere)
  (params (OverlappedComponent :type Primitive%20Component%20Object%20Reference) (OtherActor :type Actor%20Object%20Reference) (OtherComp :type Primitive%20Component%20Object%20Reference) (OtherBodyIndex :type Integer))
  (bind _asbp_enemy_parent (Utilities|Casting|CastToBP_EnemyParent OtherActor))
  (Utilities|Array|RemoveItem (Variables|Default|GetEnemiesInRange) _asbp_enemy_parent))

(event Custom|Fire
  (bind _enemiesinrange (Variables|Default|GetEnemiesInRange))
  (if (> (Utilities|Array|Length (Variables|Default|GetEnemiesInRange)) 0)
    (bind _output_get (Variables|Default|SetCurrentTarget (Utilities|Array|Get(acopy) _enemiesinrange)))
    (if (Utilities|IsValid _output_get)
      (if (Utilities|Array|ContainsItem _enemiesinrange _output_get)
        (bind _asbp_enemy_parent (Utilities|Casting|CastToBP_EnemyParent _output_get))
        (Transformation|SetActorRotation (Math|Rotator|FindLookatRotation (Transformation|GetActorLocation) (Transformation|GetActorLocation _asbp_enemy_parent)))
        (Game|SpawnActorfromClass "/Game/Actors/BP_Projectile.BP_Projectile_C" (Math|Transform|MakeTransform (+ (Transformation|GetActorLocation) "0.000000,0.000000,50.000000") (Transformation|GetActorRotation)) "Undefined" "MultiplyWithRoot" 0 (Variables|Default|GetDamage) _asbp_enemy_parent 0)))))

(event EventBeginPlay
  (Utilities|Time|SetTimerbyFunctionName 0 "Fire" (Variables|Default|GetFireRate) true))

(event Collision|EventActorBeginOverlap
  (params (OtherActor :type Actor%20Object%20Reference))
  (|CallParentFunction OtherActor) ; This node is disabled and will not be called.\nDrag off pins to build functionality.
)

(event EventTick
  (params (DeltaSeconds :type Float%20%28single-precision%29)))

(fn ConstructionScript
  (|CallParentFunction))